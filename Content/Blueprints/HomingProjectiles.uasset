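; A physics-driven projectile actor, intended as a homing missile, that explodes and destroys itself on hit.
; BeginPlay caches the first found target actor; Tick drives component E at constant forward speed, setting angular velocity from the player-to-projectile look-at direction rather than the target's position.
; Hits spawn an explosion, adding a collapse sound if the target was struck.
; Timer, impulse and homing-component setups are unconnected leftovers.
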(event OnComponentHit(e)
  (params (HitComponent :type Primitive%20Component%20Object%20Reference) (OtherActor :type Actor%20Object%20Reference) (OtherComp :type Primitive%20Component%20Object%20Reference) (NormalImpulse :type Vector :default "0, 0, 0") (Hit :type Hit%20Result%20Structure%20%28by%20ref%29))
  (Utilities|FlowControl|Sequence
    (:then_0
      (if (== (Variables|Default|GetTarget_) OtherActor)
        (Audio|PlaySoundatLocation "/Game/StarterContent/Audio/Collapse01.Collapse01" (Variables|Default|GetNewVar_0) "0, 0, 0" 1.0 1.0 0.0 0 0 0)))
    (:then_1
      (Effects|SpawnEmitteratLocation "/Game/StarterContent/Particles/P_Explosion.P_Explosion" (.location Hit))
      (Actor|DestroyActor))))

(event Custom|Move%20to%20targer
  (Utilities|IsValid (Variables|Default|GetTarget_)))

(event Collision|EventActorBeginOverlap
  (params (OtherActor :type Actor%20Object%20Reference)))

(event EventTick
  (params (DeltaSeconds :type Float%20%28single-precision%29))
  (bind _e (Variables|Default|Gete))
  (Utilities|IsValid _e
    (:Is%20Valid
      (Utilities|IsValid (Variables|Default|GetTarget_)
        (:Is%20Valid
          (Class|PrimitiveComponent|SetPhysicsAngularVelocityinDegrees _e (Math|Rotator|GetRotationXVector (Math|Rotator|FindLookatRotation (Transformation|GetActorLocation (Game|GetPlayerCharacter 0)) (Transformation|GetActorLocation))) false "None")
          (Physics|SetPhysicsLinearVelocity _e (* (Math|Vector|GetForwardVector (Variables|Default|Gete self)) 300) false "None"))
        (:Is%20Not%20Valid
          (Physics|SetPhysicsLinearVelocity _e (* (Transformation|GetActorForwardVector self) 3e+02) false "None"))))))

(event EventBeginPlay
  (bind _outactors (Actor|GetAllActorsOfClass "/Game/Blueprints/Target.Target_C"))
  (Variables|Default|SetTarget_ (Utilities|Array|Get(acopy) _outactors)))

(fn ConstructionScript)
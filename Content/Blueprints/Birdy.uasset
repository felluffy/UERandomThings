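; Birdy is a bird actor that flaps upward on a physics-driven static mesh when Space or the SpaceButtonBla event fires.
; Each flap prints a debug "Hello" and applies a velocity-change impulse from the actor's up vector, scaled only on Z.
; Tick draws a debug sphere trace along velocity, leaving its result unused, and adds the look-at rotation toward velocity as a relative offset each frame.
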(event Custom|SpaceButtonBla
  (bind _returnvalue (Transformation|GetActorUpVector))
  (bind _returnvalue_2 (Math|Vector|Normalize _returnvalue))
  (Development|PrintText "Hello")
  (Physics|AddImpulse (Variables|Default|GetStaticMesh) (Math|Vector|MakeVector (.x _returnvalue_2) (.y _returnvalue_2) (* (.z _returnvalue_2) 6e+02)) "None" true))

(event EventBeginPlay)

(event Collision|EventActorBeginOverlap
  (params (OtherActor :type Actor%20Object%20Reference)))

(event EventTick
  (params (DeltaSeconds :type Float%20%28single-precision%29))
  (bind _returnvalue (Transformation|GetVelocity))
  (bind _staticmesh (Variables|Default|GetStaticMesh))
  (bind _returnvalue_2 (Transformation|GetWorldLocation _staticmesh))
  (bind _returnvalue_3 (+ _returnvalue _returnvalue_2))
  (Collision|SphereTraceByChannel _returnvalue_2 _returnvalue_3 2e+01 "TraceTypeQuery1" false 0 "ForOneFrame")
  (Transformation|AddRelativeRotation (Variables|Default|GetStaticMesh) (Math|Rotator|FindLookatRotation _returnvalue_2 _returnvalue_3) false false))

(event Input|KeyboardEvents|SpaceBar
  (params (Key :type Key%20Structure :default "None"))
  (bind _returnvalue (Transformation|GetActorUpVector))
  (bind _returnvalue_2 (Math|Vector|Normalize _returnvalue))
  (:Pressed
    (Development|PrintText "Hello")
    (Physics|AddImpulse (Variables|Default|GetStaticMesh) (Math|Vector|MakeVector (.x _returnvalue_2) (.y _returnvalue_2) (* (.z _returnvalue_2) 6e+02)) "None" true)))

(event Input|KeyboardEvents|Left
  (params (Key :type Key%20Structure :default "None")))

(fn ConstructionScript)
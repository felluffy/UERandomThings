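; Test actor with a spotlight that wanders over a target actor while its color and cone shape drift at random.
; BeginPlay sets a random color and starts a looping timer that picks a new random color, cone angles and look-at rotation toward a random point within the target's bounds.
; Tick eases the light toward those values with interpolation, giving slow, continuous motion instead of jumps.
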(event Custom|Light
  (bind _targetref (Variables|Default|GetTargetRef))
  (bind (_origin _boxextent) (Collision|GetActorBounds _targetref false))
  (bind _output_get (Variables|Default|SetInnerNew (Math|Random|RandomFloatinRange 1.0 15.0)))
  (Variables|Default|SetOuterNew (Math|Random|RandomFloatinRange _output_get (+ _output_get 15.0)))
  (Variables|Default|SetNewRot (Math|Rotator|FindLookatRotation (Transformation|GetActorLocation) (Math|Random|RandomPointinBoundingBox _origin (Math|Vector|MakeVector (.x _boxextent) (.y _boxextent) (.z _boxextent)))))
  (Variables|Default|SetColor (Math|Vector|MakeVector (Math|Random|RandomFloatinRange 0.1 0.9) (Math|Random|RandomFloatinRange 0.1 0.9) (Math|Random|RandomFloatinRange 0.1 0.9))))

(event EventBeginPlay
  (bind _returnvalue (Math|Random|RandomFloatinRange 0.0 1.0))
  (bind _returnvalue_2 (Math|Random|RandomFloatinRange 0.0 1.0))
  (bind _returnvalue_3 (Math|Random|RandomFloatinRange 0.0 1.0))
  (bind _returnvalue_4 (Math|Vector|MakeVector _returnvalue _returnvalue_2 _returnvalue_3))
  (Variables|Default|SetColor _returnvalue_4)
  (Rendering|Components|Light|SetLightColor (Variables|Default|GetSpotLight) (Math|Conversions|ToLinearColor(Vector) _returnvalue_4) true)
  (Utilities|Time|SetTimerbyEvent (delegate Custom|Light) 1.0 true 0.1))

(event Collision|EventActorBeginOverlap
  (params (OtherActor :type Actor%20Object%20Reference)))

(event EventTick
  (params (DeltaSeconds :type Float%20%28single-precision%29))
  (bind _spotlight (Variables|Default|GetSpotLight))
  (bind _spotlight_2 (Variables|Default|GetSpotLight))
  (bind _color (Variables|Default|GetColor))
  (bind _spotlight_3 (Variables|Default|GetSpotLight))
  (bind _spotlight_4 (Variables|Default|GetSpotLight))
  (bind _returnvalue (Rendering|Components|Light|GetLightColor _spotlight_4))
  (Transformation|SetWorldRotation _spotlight_3 (Math|Interpolation|RInterpTo (Transformation|GetWorldRotation _spotlight_3) (Variables|Default|GetNewRot) DeltaSeconds 0.5) false false)
  (Rendering|Lighting|SetInnerConeAngle _spotlight_2 (Math|Interpolation|FInterpTo (Variables|/Script/Engine.SpotLightComponent|GetInnerConeAngle _spotlight) (Variables|Default|GetInnerNew) DeltaSeconds 0.5))
  (Rendering|Lighting|SetOuterConeAngle _spotlight_2 (Math|Interpolation|FInterpTo (Variables|/Script/Engine.SpotLightComponent|GetOuterConeAngle _spotlight) (Variables|Default|GetOuterNew) DeltaSeconds 0.5))
  (Rendering|Components|Light|SetLightColor _spotlight_4 (Math|Color|MakeColor (Math|Interpolation|FInterpTo (.r _returnvalue) (.x _color) DeltaSeconds 1.0) (Math|Interpolation|FInterpTo (.g _returnvalue) (.y _color) DeltaSeconds 1.0) (Math|Interpolation|FInterpTo (.b _returnvalue) (.z _color) DeltaSeconds 1.0)) true))

(fn ConstructionScript)
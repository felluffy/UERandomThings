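; Test homing projectile that chases the player pawn and explodes on impact.
; Tick eases rotation toward the player and applies the normalized world direction as an unswept local offset, a fixed step independent of frame time.
; Sphere hits spawn an explosion and destroy the actor, adding a sound if they hit the Target found at BeginPlay.
; Impulse and projectile-homing experiments remain disconnected.
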(event OnComponentHit(Sphere)
  (params (HitComponent :type Primitive%20Component%20Object%20Reference) (OtherActor :type Actor%20Object%20Reference) (OtherComp :type Primitive%20Component%20Object%20Reference) (NormalImpulse :type Vector :default "0, 0, 0") (Hit :type Hit%20Result%20Structure%20%28by%20ref%29))
  (Utilities|FlowControl|Sequence
    (:then_0
      (if (== (Variables|Default|GetTarget_) OtherActor)
        (Audio|PlaySoundatLocation "/Game/StarterContent/Audio/Collapse01.Collapse01" (Variables|Default|GetNewVar_0) "0, 0, 0" 1.0 1.0 0.0 0 0 0)))
    (:then_1
      (Effects|SpawnEmitteratLocation "/Game/StarterContent/Particles/P_Explosion.P_Explosion" (Transformation|GetActorLocation))
      (Actor|DestroyActor))))

(event Custom|Move%20to%20targer
  (Utilities|IsValid (Variables|Default|GetTarget_)))

(event Collision|EventActorBeginOverlap
  (params (OtherActor :type Actor%20Object%20Reference)))

(event EventTick
  (params (DeltaSeconds :type Float%20%28single-precision%29))
  (bind _returnvalue (Transformation|GetActorLocation))
  (bind _returnvalue_2 (Game|Player|GetPlayerPawn 0))
  (bind _returnvalue_3 (Transformation|GetActorLocation _returnvalue_2))
  (Transformation|SetActorRotation self (Math|Interpolation|RInterpTo (Transformation|GetActorRotation) (Math|Rotator|FindLookatRotation _returnvalue _returnvalue_3) DeltaSeconds 1.2))
  (Transformation|AddActorLocalOffset (* (Math|Vector|Normalize (- _returnvalue_3 _returnvalue)) 5e+01) false false))

(event EventBeginPlay
  (bind _outactors (Actor|GetAllActorsOfClass "/Game/Blueprints/Target.Target_C"))
  (Variables|Default|SetTarget_ (Utilities|Array|Get(acopy) _outactors)))

(fn ConstructionScript)
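; Projectile actor that seeds a secondary burst of projectiles where it hits.
; On begin play it prints its owner's name and turns off move-ignore for owner and instigator.
; The first hit on anything but the instigator spawns a PostBlastSpawner, passing it the impact normal and projectile count.
; Each such hit also deactivates the particle system and draws a debug line and cone along the normal.
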(event OnComponentHit(CollisionComponent)
  (params (HitComponent :type Primitive%20Component%20Object%20Reference) (OtherActor :type Actor%20Object%20Reference) (OtherComp :type Primitive%20Component%20Object%20Reference) (NormalImpulse :type Vector :default "0, 0, 0") (Hit :type Hit%20Result%20Structure%20%28by%20ref%29))
  (if (!= OtherActor (Game|GetInstigator))
    (Utilities|FlowControl|Sequence
      (:then_0
        (if (Math|Boolean|Equal(Boolean) (Variables|Default|Getdoonce) false)
          (Variables|Default|Setdoonce true)
          (bind _returnvalue (Game|SpawnActorfromClass "/Game/Blueprints/BoxStuff/PostBlastSpawner.PostBlastSpawner_C" (Math|Transform|MakeTransform (.location Hit) "0, 0,0.000000") "Undefined" (Components|GetOwner) (Game|GetInstigator)))
          (Default|SetVals _returnvalue (.impactnormal Hit) 15)))
      (:then_1
        (Components|Activation|Deactivate (Variables|Default|GetParticleSystem))
        (Rendering|Debug|DrawDebugLine :LineStart (.impactpoint Hit) :LineEnd (+ (.impactpoint Hit) (* (.impactnormal Hit) 2e+02)) :Duration 1e+01 :Thickness 4.0)
        (Class|KismetSystemLibrary|DrawDebugConeinDegrees (.impactpoint Hit) (.impactnormal Hit) 1e+02 45.0 45.0 12 "(R=1.000000,G=1.000000,B=1.000000,A=1.000000)" 4.0 4.0)))))

(event EventBeginPlay
  (bind _returnvalue (Components|GetOwner))
  (Development|PrintText (Utilities|Text|ToText(String) (Utilities|GetObjectName _returnvalue)))
  (Collision|IgnoreActorwhenMoving (Variables|Default|GetCollisionComponent) _returnvalue false)
  (Collision|IgnoreActorwhenMoving (Variables|Default|GetCollisionComponent) (Game|GetInstigator) false))

(event Collision|EventActorBeginOverlap
  (params (OtherActor :type Actor%20Object%20Reference)))

(event EventTick
  (params (DeltaSeconds :type Float%20%28single-precision%29)))

(fn ConstructionScript)
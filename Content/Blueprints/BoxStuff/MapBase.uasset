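; MapBase is an actor that builds a grid map of BoxAnother actors when play begins.
; Nested Rows and Columns loops, inclusive of both ends, spawn boxes spaced by SeperatorAmount from its own location, always spawning despite collisions.
; If both WorldOutlinerBot and WorldOutlinerTop are valid, it then moves them to opposite corners of the grid, half a spacing outside and raised above it.
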(event EventBeginPlay
  (bind _returnvalue (Transformation|GetActorLocation))
  (bind _returnvalue_2 (Transformation|GetActorLocation))
  (bind _returnvalue_3 (Transformation|GetActorLocation))
  (bind _worldoutliner_bot (Variables|Default|GetWorldOutliner_Bot))
  (bind _seperatoramount (Variables|Default|GetSeperatorAmount))
  (bind _seperatoramount_2 (Variables|Default|GetSeperatorAmount))
  (bind _returnvalue_4 (/ _seperatoramount 2.0))
  (bind _returnvalue_5 (/ _seperatoramount_2 2.0))
  (bind _returnvalue_6 (+ (.z _returnvalue) 1e+02))
  (for _index (range 0 (Variables|Default|GetRows))
    (for _index_2 (range 0 (Variables|Default|GetColumns))
      (Game|SpawnActorfromClass "/Game/Blueprints/BoxStuff/BoxAnother.BoxAnother_C" (Math|Transform|MakeTransform (Math|Vector|MakeVector (+ (.x _returnvalue_2) (* _index (Variables|Default|GetSeperatorAmount))) (+ (.y _returnvalue_2) (* _index_2 (Variables|Default|GetSeperatorAmount))) (.z _returnvalue_2)) "0, 0, 0" "1,1,1") "AlwaysSpawn" self 0)))
  (if (and (Utilities|IsValid (Variables|Default|GetWorldOutliner_Top)) (Utilities|IsValid _worldoutliner_bot))
    (Transformation|SetActorLocation _worldoutliner_bot (Math|Vector|MakeVector (- (.x _returnvalue_3) _returnvalue_5) (- (.y _returnvalue_3) _returnvalue_5) _returnvalue_6) false false)
    (Transformation|SetActorLocation (Variables|Default|GetWorldOutliner_Top) (Math|Vector|MakeVector (+ (* (- (Variables|Default|GetRows) 0) (Variables|Default|GetSeperatorAmount)) (.x _returnvalue) _returnvalue_4) (+ (.y _returnvalue) (* (- (Variables|Default|GetColumns) 0) (Variables|Default|GetSeperatorAmount)) _returnvalue_4) _returnvalue_6) false false)))

(event Collision|EventActorBeginOverlap
  (params (OtherActor :type Actor%20Object%20Reference)))

(event EventTick
  (params (DeltaSeconds :type Float%20%28single-precision%29)))

(fn ConstructionScript)
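; BoxChar is a player-controlled test character with axis movement, mouse yaw and an inventory of weapons.
; BeginPlay spawns two test weapons into InventoryComponent, which the mouse wheel cycles with debug prints.
; Left mouse press and release forward to the current item as a WeaponBase, while older equip logic sits unconnected.
; The construction script positions the camera from summed, scaled WorldOutliner actor locations and gives it a fixed rotation.
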(event EventBeginPlay
  (bind _returnvalue (Transformation|GetActorTransform))
  (bind _returnvalue_2 (Transformation|GetActorTransform))
  (bind _self self)
  (bind _self_2 self)
  (bind _returnvalue_3 (Game|SpawnActorfromClass "/Game/Blueprints/BoxStuff/TestWeap.TestWeap_C" (Math|Transform|MakeTransform (+ (.location _returnvalue_2) "0,50.000000, 0") (.rotation _returnvalue_2) (.scale _returnvalue_2)) "AlwaysSpawn" _self_2 _self_2))
  (Class|InventoryComponent|AddItemtoInventory (Variables|Components|GetInventoryComponent) _returnvalue_3)
  (bind _returnvalue_4 (Game|SpawnActorfromClass "/Game/Blueprints/BoxStuff/TestWeap_2.TestWeap_2_C" (Math|Transform|MakeTransform (+ (.location _returnvalue) "0,-50.000000, 0") (.rotation _returnvalue) (.scale _returnvalue)) "AlwaysSpawn" _self _self))
  (Class|InventoryComponent|AddItemtoInventory (Variables|Components|GetInventoryComponent) _returnvalue_4)
  (Transformation|AttachActorToActor _self_2 _self_2 "None" "KeepRelative" "KeepRelative" "KeepRelative" true))

(event Collision|EventActorBeginOverlap
  (params (OtherActor :type Actor%20Object%20Reference)))

(event EventTick
  (params (DeltaSeconds :type Float%20%28single-precision%29)))

(event Input|AxisEvents|InputAxisMoveForward
  (params (AxisValue :type Float%20%28single-precision%29))
  (bind _self self)
  (Pawn|Input|AddMovementInput _self (Transformation|GetActorForwardVector _self) AxisValue true))

(event Input|AxisEvents|InputAxisMoveRight
  (params (AxisValue :type Float%20%28single-precision%29))
  (bind _self self)
  (Pawn|Input|AddMovementInput _self (Transformation|GetActorRightVector _self) AxisValue true))

(event Input|MouseEvents|MouseX
  (params (AxisValue :type Float%20%28single-precision%29))
  (Pawn|Input|AddControllerYawInput AxisValue))

(event Input|KeyboardEvents|W
  (params (Key :type Key%20Structure :default "None")))

(event Input|MouseEvents|LeftMouseButton
  (params (Key :type Key%20Structure :default "None"))
  (bind _inventorycomponent (Variables|Components|GetInventoryComponent))
  (bind _returnvalue (Class|InventoryComponent|GetCurrentItem _inventorycomponent))
  (:Pressed
    (Utilities|IsValid _returnvalue
      (:Is%20Valid
        (bind _asweapon_base (Utilities|Casting|CastToWeaponBase _returnvalue))
        (Class|PickUps|OnPressMainButton _asweapon_base)
        (Development|PrintText "Hello" :!label _label))))
  (:Released
    (Utilities|IsValid _returnvalue
      (:Is%20Valid
        (bind _asweapon_base_2 (Utilities|Casting|CastToWeaponBase _returnvalue))
        (Class|PickUps|OnReleaseMainButton _asweapon_base_2)
        (goto _label)))))

(event Input|MouseEvents|MouseWheelUp
  (params (Key :type Key%20Structure :default "None"))
  (bind _inventorycomponent (Variables|Components|GetInventoryComponent))
  (:Pressed
    (Class|InventoryComponent|NextIteminInventory _inventorycomponent)
    (Development|PrintText (Utilities|Text|ToText(String) (Utilities|GetObjectName (Class|InventoryComponent|GetCurrentItem _inventorycomponent))))
    (bind _returnvalue (Class|InventoryComponent|GetInventoryItems (Variables|Components|GetInventoryComponent)))
    (Development|PrintText (Utilities|Text|ToText(Integer) _returnvalue))))

(event Input|MouseEvents|MouseWheelDown
  (params (Key :type Key%20Structure :default "None"))
  (bind _inventorycomponent (Variables|Components|GetInventoryComponent))
  (:Pressed
    (Class|InventoryComponent|PreviousIteminInventory _inventorycomponent)
    (Development|PrintText (Utilities|Text|ToText(String) (Utilities|GetObjectName (Class|InventoryComponent|GetCurrentItem _inventorycomponent))))
    (bind _returnvalue (Class|InventoryComponent|GetInventoryItems (Variables|Components|GetInventoryComponent)))
    (Development|PrintText (Utilities|Text|ToText(Integer) _returnvalue))))

(fn ConstructionScript
  (bind _camera (Variables|Components|GetCamera))
  (bind _outactors (Actor|GetAllActorsOfClass "/Game/Blueprints/BoxStuff/WorldOutliner.WorldOutliner_C"))
  (for _array_element _outactors
    (LocalVariables|SetLocation (+ (LocalVariables|GetLocation) (Transformation|GetActorLocation _array_element))))
  (Transformation|SetWorldLocation _camera (/ (LocalVariables|GetLocation) "2.000000,2.000000,0.050000") false false)
  (Transformation|SetWorldRotation _camera "-90.000000,0.000000, 0" false false))
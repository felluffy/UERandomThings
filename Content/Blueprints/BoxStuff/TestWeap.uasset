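; TestWeap is a test weapon Blueprint that drives a particle beam from the actor.
; BeginPlay adds a particle system component, and Tick sets its first emitter's beam end point to 1000 units along the actor's right vector.
; Disconnected experiments remain for muzzle smoke, snapping the weapon mesh to the overlap sphere, and a random-cone line trace, none of which run.
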(event EventBeginPlay
  (bind _returnvalue (AddComponent|AddParticleSystemComponent false)))

(event Collision|EventActorBeginOverlap
  (params (OtherActor :type Actor%20Object%20Reference)))

(event EventTick
  (params (DeltaSeconds :type Float%20%28single-precision%29))
  (Class|ParticleSystemComponent|SetBeamEndPoint (stale EventBeginPlay _returnvalue) 0 (+ (Transformation|GetActorLocation) (* (Transformation|GetActorRightVector self) 1000))))

(fn ConstructionScript)
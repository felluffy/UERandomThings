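; BoxAnother is an actor whose cube changes height in response to the mass and proximity of nearby projectiles and balls.
; A radius-sized sphere tracks overlapping TProjectile and balls actors in a map keyed to their mass.
; Each Tick sums mass over MaxWeight, weighted by horizontal distance falloff, clamps the total, and eases the cube's Z scale toward it with FInterpTo.
; The random SetScales event and several disconnected chains are unused.
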(event OnComponentBeginOverlap(Sphere)
  (params (OverlappedComponent :type Primitive%20Component%20Object%20Reference) (OtherActor :type Actor%20Object%20Reference) (OtherComp :type Primitive%20Component%20Object%20Reference) (OtherBodyIndex :type Integer) (bFromSweep :type Boolean) (SweepResult :type Hit%20Result%20Structure%20%28by%20ref%29))
  (Utilities|FlowControl|Sequence
    (:then_0
      (bind _astprojectile (Utilities|Casting|CastToTProjectile OtherActor))
      (bind _returnvalue (Class|TProjectile|GetProjectileMass _astprojectile))
      (Utilities|Map|Add (Variables|Default|GetMAP_) _astprojectile _returnvalue))
    (:then_1
      (bind _asballs (Utilities|Casting|CastToballs OtherActor))
      (Utilities|Map|Add (Variables|Default|GetMAP_) _asballs (Physics|GetMass (Variables|/Game/Blueprints/BoxStuff/balls.balls_C|GetStaticProj _asballs))))))

(event OnComponentEndOverlap(Sphere)
  (params (OverlappedComponent :type Primitive%20Component%20Object%20Reference) (OtherActor :type Actor%20Object%20Reference) (OtherComp :type Primitive%20Component%20Object%20Reference) (OtherBodyIndex :type Integer))
  (bind _map_ (Variables|Default|GetMAP_))
  (if (Utilities|Map|Contains _map_ OtherActor)
    (Utilities|Map|Remove _map_ OtherActor)))

(event Custom|SetScales
  (Variables|Default|SetNewScale (Math|Vector|MakeVector 1.0 1.0 (Math|Random|RandomFloatinRange 2.0 0.1))))

(event EventBeginPlay
  (Components|Sphere|SetSphereRadius (Variables|Default|GetSphere) (Variables|Default|GetRadius) true))

(event Collision|EventActorBeginOverlap
  (params (OtherActor :type Actor%20Object%20Reference)))

(event EventTick
  (params (DeltaSeconds :type Float%20%28single-precision%29))
  (bind _returnvalue (Transformation|GetActorLocation))
  (bind _radius (Variables|Default|GetRadius))
  (bind _map_ (Variables|Default|GetMAP_))
  (bind _cube1 (Variables|Default|GetCube1))
  (Variables|Default|SetNew_Z 0.0)
  (Utilities|FlowControl|Sequence
    (:then_0
      (bind _keys (Utilities|Map|Keys _map_))
      (for _array_element _keys
        (Variables|Default|SetNew_Z (+ (Variables|Default|GetNew_Z) (* (/ (.Value (Utilities|Map|Find _map_ _array_element)) (Variables|Default|GetMaxWeight)) (/ (- _radius (* 5 (Math|Vector|Distance2D(Vector) (Math|Vector2D|MakeVector2D (.x _returnvalue) (.y _returnvalue)) (Math|Vector2D|MakeVector2D (.x (Transformation|GetActorLocation _array_element)) (.y (Transformation|GetActorLocation _array_element)))))) _radius)) 0.0)))
      (Variables|Default|SetNewScale (Math|Vector|MakeVector 1.0 1.0 (Math|Float|Clamp(Float) (Variables|Default|GetNew_Z) 0.1))))
    (:then_1
      (Transformation|SetWorldScale3D _cube1 (Math|Vector|MakeVector 1.0 1.0 (Math|Interpolation|FInterpTo (.z (Transformation|GetWorldScale _cube1)) (.z (Variables|Default|GetNewScale)) DeltaSeconds 1.0))))))

(fn ConstructionScript)
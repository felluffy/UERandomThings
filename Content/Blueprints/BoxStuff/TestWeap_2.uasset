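; Test weapon Blueprint that displays the SK_AR4_X skeletal mesh, with no active gameplay logic.
; The construction script snaps WeaponMesh to the OverlapSphere's location and assigns that mesh.
; The event graph holds only empty events and unconnected drafts of a random-cone debug line trace and a camera shake.
; The draft trace's end point is not offset from the actor's location.
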(event EventBeginPlay)

(event Collision|EventActorBeginOverlap
  (params (OtherActor :type Actor%20Object%20Reference)))

(event EventTick
  (params (DeltaSeconds :type Float%20%28single-precision%29)))

(fn ConstructionScript
  (Transformation|SetWorldLocation (Variables|Default|GetWeaponMesh) (Transformation|GetWorldLocation (Variables|Default|GetOverlapSphere)) false false)
  (Class|SkinnedMeshComponent|SetSkeletalMesh (Variables|Default|GetWeaponMesh) "/Game/FPS_Weapon_Bundle/Weapons/Meshes/AR4/SK_AR4_X.SK_AR4_X" true))
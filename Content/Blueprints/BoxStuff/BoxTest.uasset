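; Test box actor that feeds the position of the nearest nearby actor into its cube's material.
; Construction creates a dynamic material instance with a random Weight, which BeginPlay re-randomizes.
; A looping 60 Hz timer sphere-overlaps WorldStatic actors, ignoring same-class actors, and writes the closest location to PositionClosest when any are found.
; An uncalled debug event and disconnected trace and print experiments remain in the graph.
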(event Custom|CustomEvent_0
  (Variables|Default|Setiter (Variables|Default|Getiter))
  (Variables|Default|Setleast_Dist 1e+05)
  (bind _outactors (Actor|GetAllActorsOfClass (Utilities|GetClass self)))
  (bind (_outactors_2 _returnvalue) (Collision|SphereOverlapActors (Transformation|GetActorLocation self) 3.5e+02 (Utilities|Array|MakeArray "ObjectTypeQuery2" "ObjectTypeQuery3" "ObjectTypeQuery1") "/Script/Engine.Actor" _outactors))
  (if _returnvalue
    (for _array_element _outactors_2
      (if (<= (Math|Vector|VectorLength (- (Transformation|GetActorLocation _array_element) (Transformation|GetActorLocation self))) (Variables|Default|Getleast_Dist))
        (bind _output_get (Variables|Default|Setleast_Dist (Math|Vector|VectorLength (- (Transformation|GetActorLocation _array_element) (Transformation|GetActorLocation self)))))))
    (Development|PrintText (Utilities|Text|ToText(String) (Utilities|String|Append (Utilities|GetObjectName _array_element) " - " (Utilities|String|ToString(Float) (Transformation|GetDistanceTo _array_element self)) " by " (Utilities|GetObjectName self))) true true "(R=0.000000,G=0.660000,B=1.000000,A=1.000000)" 0.3)))

(event Custom|LAAlA
  (Variables|Default|Setleast_Dist 1e+03)
  (Variables|Default|SetClosestDistance "10000001.000000,10000.000000,10000.000000")
  (bind (_outactors _returnvalue) (Collision|SphereOverlapActors (Transformation|GetActorLocation) 3e+02 (Utilities|Array|MakeArray "ObjectTypeQuery1") "/Script/Engine.Actor" (Variables|Default|GetIgnore)))
  (if _returnvalue
    (for _array_element _outactors
      (if (<= (Math|Vector|VectorLength (- (Transformation|GetActorLocation _array_element) (Transformation|GetActorLocation self))) (Variables|Default|Getleast_Dist))
        (Variables|Default|Setleast_Dist (Math|Vector|VectorLength (- (Transformation|GetActorLocation _array_element) (Transformation|GetActorLocation self))))
        (Variables|Default|SetClosestDistance (Transformation|GetActorLocation _array_element))))
    (Rendering|Material|SetVectorParameterValue (Variables|Default|GetMat_inst) "PositionClosest" (Math|Conversions|ToLinearColor(Vector) (Variables|Default|GetClosestDistance)) :!class /Script/Engine.MaterialInstanceDynamic)))

(event EventBeginPlay
  (Rendering|Material|SetScalarParameterValue (Variables|Default|GetMat_inst) "Weight" (Math|Random|RandomFloatinRange -1.0 1.0) :!class /Script/Engine.MaterialInstanceDynamic)
  (bind _outactors (Actor|GetAllActorsOfClass (Utilities|GetClass self)))
  (Variables|Default|SetIgnore _outactors)
  (Utilities|Time|SetTimerbyEvent (delegate Custom|LAAlA) 0.01667 true 0.1))

(event Collision|EventActorBeginOverlap
  (params (OtherActor :type Actor%20Object%20Reference)))

(event EventTick
  (params (DeltaSeconds :type Float%20%28single-precision%29)))

(fn ConstructionScript
  (bind _returnvalue (Rendering|Material|CreateDynamicMaterialInstance (Variables|Default|GetCube) 0 "/Game/Materials/ShapeBox_dup_Inst.ShapeBox_dup_Inst" "None" :!class /Script/Engine.PrimitiveComponent))
  (bind _output_get (Variables|Default|SetMat_inst _returnvalue))
  (Rendering|Material|SetScalarParameterValue _output_get "Weight" (Math|Random|RandomFloatinRange -1.0 1.0) :!class /Script/Engine.MaterialInstanceDynamic)
  (Rendering|Material|SetVectorParameterValue (Variables|Default|GetMat_inst) "PositionClosest" (Math|Conversions|ToLinearColor(Vector) "10000.000000,10000.000000,10000.000000") :!class /Script/Engine.MaterialInstanceDynamic))
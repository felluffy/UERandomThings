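; PostBlastSpawner is an actor that throws a burst of small, randomly scaled Balls, then destroys itself.
; A BeginPlay timer calls SetVals with its up vector and a count; though looping, self-destruction ends it after one burst.
; Each ball gets an impulse within a cone around that normal and ignores the spawner's owner when moving.
; The loop's trailing Delay does not stagger spawns.
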(event Custom|SetVals
  (params (ImpactNormal :type Vector) (NumProjsToSpawn :type Integer))
  (Variables|Default|SetImpactNormal ImpactNormal)
  (bind _output_get (Variables|Default|SetNumProjsToSpawn NumProjsToSpawn))
  (for _index (range 0 _output_get)
    (bind _returnvalue (Game|SpawnActorfromClass "/Game/Blueprints/BoxStuff/balls.balls_C" (Math|Transform|MakeTransform (Transformation|GetWorldLocation (Variables|Default|GetDefaultSceneRoot self)) (Math|Rotator|MakeRotfromX (Math|Random|RandomUnitVectorinConeinDegrees (Variables|Default|GetImpactNormal) 3e+01)) (Math|Vector|MakeVector (Math|Random|RandomFloatinRange 0.05 0.1) (Math|Random|RandomFloatinRange 0.05 0.1) (Math|Random|RandomFloatinRange 0.05 0.1))) "AlwaysSpawn" (Components|GetOwner) (Game|GetInstigator)))
    (Physics|AddImpulse (Variables|/Game/Blueprints/BoxStuff/balls.balls_C|GetStaticProj _returnvalue) (* (Math|Random|RandomUnitVectorinConeinDegrees (Variables|Default|GetImpactNormal) 3e+01) 1000) "None" true)
    (Collision|IgnoreActorwhenMoving (Variables|/Game/Blueprints/BoxStuff/balls.balls_C|GetStaticProj _returnvalue) (Components|GetOwner) true)
    (Utilities|FlowControl|Delay 0.1))
  (Actor|DestroyActor))

(event Custom|FDFDS
  (CallFunction|SetVals (Transformation|GetActorUpVector self) 15))

(event EventBeginPlay
  (Utilities|Time|SetTimerbyEvent (delegate Custom|FDFDS) 2.0 true 0.1))

(event Collision|EventActorBeginOverlap
  (params (OtherActor :type Actor%20Object%20Reference)))

(event EventTick
  (params (DeltaSeconds :type Float%20%28single-precision%29)))

(fn ConstructionScript)